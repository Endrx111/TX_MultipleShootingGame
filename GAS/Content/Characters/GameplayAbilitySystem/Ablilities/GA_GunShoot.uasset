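; GA_GunShoot is an event-activated gameplay ability that applies bullet damage to the actor a shot hits.
; On activation it applies GE_BulletHit to the event's Target if that has an ability system component, passing Damage as a SetByCaller magnitude on Data.Damage, then ends.
; A CastDamage event repeats this on HitActor behind an authority check, with no caller in this graph.
; The Character.Killer event send is disconnected.
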(event Custom|CastDamage
  (bind _hit_actor (Variables|Default|GetHit%20Actor))
  (bind _returnvalue (Ability|GetAbilitySystemComponent _hit_actor))
  (Ability|HasAuthority
    (:True
      (Utilities|IsValid _returnvalue
        (:Is%20Valid
          (bind _returnvalue_2 (Ability|GameplayEffect|AssignTagSetbyCallerMagnitude (Ability|MakeOutgoingGameplayEffectSpec "/Game/Characters/GameplayAbilitySystem/Effect/GE_BulletHit.GE_BulletHit_C") "(TagName=\"Data.Damage\")" (Variables|Default|GetDamage)))
          (GameplayEffects|ApplyGameplayEffectSpecToSelf _returnvalue _returnvalue_2))))))

(event Ability|EventActivateAbilityFromEvent
  (params (EventData :type Gameplay%20Event%20Data%20Structure%20%28by%20ref%29))
  (bind (_eventtag _instigator _target _optionalobject _optionalobject2 _contexthandle _instigatortags _targettags _eventmagnitude _targetdata) (Utilities|Struct|BreakGameplayEventData EventData))
  (bind _returnvalue (Ability|GetAbilitySystemComponent _target))
  (Utilities|IsValid _returnvalue
    (:Is%20Valid
      (bind _returnvalue_2 (Ability|GameplayEffect|AssignTagSetbyCallerMagnitude (Ability|MakeOutgoingGameplayEffectSpec "/Game/Characters/GameplayAbilitySystem/Effect/GE_BulletHit.GE_BulletHit_C") "(TagName=\"Data.Damage\")" (Variables|Default|GetDamage)))
      (GameplayEffects|ApplyGameplayEffectSpecToSelf _returnvalue _returnvalue_2)
      (Ability|EndAbility self))
    (:Is%20Not%20Valid
      (Ability|EndAbility))))