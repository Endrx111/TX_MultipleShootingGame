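; Gameplay ability that equips or unequips the avatar's weapon when activated by a gameplay event.
; After committing, it switches on the event's first target tag and calls the avatar's WeaponsManagerComponent before ending.
; The Virtus tag equips BP_Phiso, Rifle equips BP_VIRTUS, and unmatched tags unequip; the Primary weapon branch is an empty stub.
; EndAbility runs only when that component is valid, and the commit result is unchecked.
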(event Ability|EventActivateAbility)

(event Ability|EventActivateAbilityFromEvent
  (params (EventData :type Gameplay%20Event%20Data%20Structure%20%28by%20ref%29))
  (bind _returnvalue (Ability|GetAvatarActorfromActorInfo))
  (bind _returnvalue_2 (Actor|GetComponentbyClass _returnvalue "/Game/Code/Weapon/WeaponsManagerComponent.WeaponsManagerComponent_C"))
  (Ability|CommitAbility)
  (Utilities|IsValid _returnvalue_2
    (:Is%20Valid
      (Utilities|FlowControl|Sequence
        (:then_0
          (|SwitchGameplayTag (Utilities|Array|Get(acopy) (GameplayTags|BreakGameplayTagContainer (.TargetTags (Utilities|Struct|BreakGameplayEventData EventData))))
            (:Default
              (Default|UnquipWeapon _returnvalue_2))
            (:Weapon.Range.Virtus
              (Default|EquipWeapon _returnvalue_2 "/Game/Code/Weapon/BP_Phiso.BP_Phiso_C" false "/Game/Code/Player/Animation/P/ABP_FPSPlayer.ABP_FPSPlayer_C"))
            (:Weapon.Range.Rifle
              (Default|EquipWeapon _returnvalue_2 "/Game/Code/Weapon/BP_VIRTUS.BP_VIRTUS_C" false "/Game/Code/Player/Animation/P/ABP_FPSPlayer.ABP_FPSPlayer_C"))
            (:Character.C_Weapon.Primary
              (|SwitchGameplayTag))))
        (:then_1
          (Ability|EndAbility))))))