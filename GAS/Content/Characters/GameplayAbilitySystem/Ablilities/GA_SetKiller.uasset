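; GA_SetKiller is a Gameplay Ability that records who killed a player.
; When activated from a gameplay event, it casts the avatar to BP_PlayerBase and passes the event's Instigator to SetKiller, printing on a failed cast.
; The live path never calls EndAbility.
; Death effect, tag-wait and death GameplayCue logic remain in the graph but are disconnected and never run.
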(event Ability|EventActivateAbility)

(event Ability|EventOnEndAbility
  (params (bWasCancelled :type Boolean)))

(event Ability|EventActivateAbilityFromEvent
  (params (EventData :type Gameplay%20Event%20Data%20Structure%20%28by%20ref%29))
  (bind _asbp_player_base (Utilities|Casting|CastToBP_PlayerBase (Ability|GetAvatarActorfromActorInfo))
    (:then
      (Default|SetKiller _asbp_player_base (.instigator EventData)))
    (:CastFailed
      (Development|PrintString "Cast Fail" true true "(R=0.000000,G=0.086702,B=0.173958,A=1.000000)"))))