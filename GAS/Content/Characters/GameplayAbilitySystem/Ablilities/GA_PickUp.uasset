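; Gameplay ability that lets the player pick up a weapon, swapping out whatever occupies that slot.
; The triggering event's first target tag selects the primary or secondary slot; if that slot is filled, DropWeapon spawns its pickup class just ahead of the player.
; It then sends INteractMessage to the first overlapping BP_PickUPBase and ends.
; The CommitAbility result only gates a debug print, and leftover reload and class-check logic never runs.
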(event Custom|DropWeapon
  (params (WeaponToDrop :type BP%20Pick%20UP%20Base%20Class%20Reference))
  (bind _as_bp_player_base (Variables|Default|GetAs%20BP%20Player%20Base))
  (bind _returnvalue (Transformation|GetActorTransform _as_bp_player_base))
  (Game|SpawnActorfromClass WeaponToDrop (Math|Transform|MakeTransform (+ (.location _returnvalue) (* (Math|Vector|GetForwardVector (.rotation _returnvalue)) 3e+01)) "0, 0, 0" "1.000000,1.000000,1.000000") "Undefined" "MultiplyWithRoot" 0 0))

(event Ability|EventOnEndAbility
  (params (bWasCancelled :type Boolean)))

(event Ability|EventActivateAbilityFromEvent
  (params (EventData :type Gameplay%20Event%20Data%20Structure%20%28by%20ref%29))
  (bind _returnvalue (Ability|CommitAbility))
  (Development|PrintString "PickUP" _returnvalue true "(R=0.058438,G=0.297392,B=0.660000,A=1.000000)")
  (bind _asbp_player_base (Utilities|Casting|CastToBP_PlayerBase (Ability|GetAvatarActorfromActorInfo)))
  (Variables|Default|SetAs%20BP%20Player%20Base _asbp_player_base)
  (|SwitchGameplayTag (Utilities|Array|Get(acopy) (GameplayTags|BreakGameplayTagContainer (.TargetTags (Utilities|Struct|BreakGameplayEventData EventData))))
    (:Character.C_Weapon.Primary
      (bind _primaryweapon (Variables|/Game/Characters/GameplayAbilitySystem/character/BP_PlayerBase.BP_PlayerBase_C|GetPrimaryWeapon (Variables|Default|GetAs%20BP%20Player%20Base))
        (:then
          (CallFunction|DropWeapon (Variables|/Game/Code/PickUP/BP_PickUPComponent.BP_PickUPComponent_C|GetPickUpClass _primaryweapon)))
        (:else
          _)))
    (:Character.C_Weapon.Second
      (bind _secondaryweapon (Variables|/Game/Characters/GameplayAbilitySystem/character/BP_PlayerBase.BP_PlayerBase_C|GetSecondaryWeapon (Variables|Default|GetAs%20BP%20Player%20Base))
        (:then
          (CallFunction|DropWeapon (Variables|/Game/Code/PickUP/BP_PickUPComponent.BP_PickUPComponent_C|GetPickUpClass _secondaryweapon)))
        (:else
          _))))
  (Class|BPInterract|INteract(Message) (Utilities|Array|Get(acopy) (Collision|GetOverlappingActors (Variables|Default|GetAs%20BP%20Player%20Base) "/Game/Code/PickUP/Base/BP_PickUPBase.BP_PickUPBase_C" :!class /Script/Engine.Actor)) (Variables|Default|GetAs%20BP%20Player%20Base))
  (Ability|EndAbility))

(fn GetWeaponClass
  (return "NewEnumerator0"))

(fn UIUpdate
  (params (GetKill :type Actor%20Object%20Reference))
  (return 0))