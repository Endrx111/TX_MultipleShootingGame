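; GA_Aim is a Gameplay Ability that, despite its aim name, calls Reload on the player's current weapon.
; It activates from a gameplay event, commits, then casts the avatar to BP_PlayerBase and checks for a WeaponsManagerComponent.
; It switches on the event's first target tag, handling only Weapon.Range.Virtus, then ends immediately.
; A failed cast or missing component leaves the ability without an EndAbility call.
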(event Ability|EventOnEndAbility
  (params (bWasCancelled :type Boolean)))

(event Ability|EventActivateAbilityFromEvent
  (params (EventData :type Gameplay%20Event%20Data%20Structure%20%28by%20ref%29))
  (bind _returnvalue (Ability|GetAvatarActorfromActorInfo))
  (Ability|CommitAbility)
  (bind _asbp_player_base (Utilities|Casting|CastToBP_PlayerBase _returnvalue))
  (Utilities|IsValid (Actor|GetComponentbyClass _returnvalue "/Game/Code/Weapon/WeaponsManagerComponent.WeaponsManagerComponent_C")
    (:Is%20Valid
      (Utilities|FlowControl|Sequence
        (:then_0
          (|SwitchGameplayTag (Utilities|Array|Get(acopy) (GameplayTags|BreakGameplayTagContainer (.TargetTags (Utilities|Struct|BreakGameplayEventData EventData))))
            (:Weapon.Range.Virtus
              (Default|Reload (Variables|/Game/Characters/GameplayAbilitySystem/character/BP_PlayerBase.BP_PlayerBase_C|GetCurrentWeapon _asbp_player_base)))))
        (:then_1
          (Ability|EndAbility))))))