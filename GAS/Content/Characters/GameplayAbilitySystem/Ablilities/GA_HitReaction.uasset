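; GA_HitReaction is a Gameplay Ability that plays a light front hit-reaction montage on its owner.
; On activation it runs a PlayMontageAndWait task with a fixed montage, then ends the ability when the montage completes, is interrupted or is cancelled.
; Disconnected leftover chains hold earlier debug prints and direct montage or animation playback on the BP_PlayerBase mesh, none of which run.
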(event Ability|EventActivateAbility
  (|PlayMontageandWaitProxy "None" "/Game/QuantumCharacter/Anims/UEMM_HitReact_Front_Lgt_01_Montage.UEMM_HitReact_Front_Lgt_01_Montage" 1.0 "None" true 1.0 0.0 false
    (:OnCompleted
      _)
    (:OnInterrupted
      _)
    (:OnCancelled
      _))
  (Ability|EndAbility))

(event Ability|EventOnEndAbility
  (params (bWasCancelled :type Boolean)))