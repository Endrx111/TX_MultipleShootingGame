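; BP_PickUPComponent is a weapon component that, on BeginPlay, installs itself as its owning BP_PlayerBase's equipped primary or secondary weapon.
; It destroys any weapon already in that slot, hides the other slot's weapon if equipped, and shows itself.
; Locally controlled players receive a GAS EquipWeapon gameplay event chosen by weapon name; otherwise it attaches to the mesh socket after a short server-latency delay.
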(event EventBeginPlay
  (bind _self self)
  (bind _socketname (Variables|Default|GetSocketName))
  (bind _asbp_player_base (Utilities|Casting|CastToBP_PlayerBase (Components|GetOwner)))
  (bind _output_get (Variables|Default|SetAs%20BP%20Player%20Base _asbp_player_base))
  (switch Utilities|FlowControl|Switch|SwitchonE_WeaponClass (Variables|Default|GetWeaponClass)
    (:NewEnumerator0
      (bind _secondaryweapon (Variables|/Game/Characters/GameplayAbilitySystem/character/BP_PlayerBase.BP_PlayerBase_C|GetSecondaryWeapon _output_get)
        (:then
          (if (== _secondaryweapon (Variables|/Game/Characters/GameplayAbilitySystem/character/BP_PlayerBase.BP_PlayerBase_C|GetEquipWeapon _output_get))
            (Rendering|SetVisibility _secondaryweapon false false)))
        (:else
          _))
      (bind _primaryweapon (Variables|/Game/Characters/GameplayAbilitySystem/character/BP_PlayerBase.BP_PlayerBase_C|GetPrimaryWeapon _asbp_player_base)
        (:then
          (Components|DestroyComponent _primaryweapon))
        (:else
          _))
      (bind _output_get_2 (Variables|/Game/Characters/GameplayAbilitySystem/character/BP_PlayerBase.BP_PlayerBase_C|SetPrimaryWeapon _asbp_player_base _self))
      (bind _output_get_3 (Variables|/Game/Characters/GameplayAbilitySystem/character/BP_PlayerBase.BP_PlayerBase_C|SetEquipWeapon _asbp_player_base _output_get_2))
      (Variables|/Game/Characters/GameplayAbilitySystem/character/BP_PlayerBase.BP_PlayerBase_C|SetCurrentWeaponInt _asbp_player_base (Math|Conversions|ToInteger(Byte) (Variables|BP_PickUPComponent_C|GetWeaponName _output_get_3)))
      (Rendering|SetVisibility (Variables|/Game/Characters/GameplayAbilitySystem/character/BP_PlayerBase.BP_PlayerBase_C|GetPrimaryWeapon _asbp_player_base) true false))
    (:NewEnumerator1
      (bind _primaryweapon_2 (Variables|/Game/Characters/GameplayAbilitySystem/character/BP_PlayerBase.BP_PlayerBase_C|GetPrimaryWeapon _output_get)
        (:then
          (if (== _primaryweapon_2 (Variables|/Game/Characters/GameplayAbilitySystem/character/BP_PlayerBase.BP_PlayerBase_C|GetEquipWeapon _output_get))
            (Rendering|SetVisibility _primaryweapon_2 false false)))
        (:else
          _))
      (bind _secondaryweapon_2 (Variables|/Game/Characters/GameplayAbilitySystem/character/BP_PlayerBase.BP_PlayerBase_C|GetSecondaryWeapon _asbp_player_base)
        (:then
          (Components|DestroyComponent _secondaryweapon_2))
        (:else
          _))
      (bind _output_get_4 (Variables|/Game/Characters/GameplayAbilitySystem/character/BP_PlayerBase.BP_PlayerBase_C|SetSecondaryWeapon _asbp_player_base _self))
      (bind _output_get_5 (Variables|/Game/Characters/GameplayAbilitySystem/character/BP_PlayerBase.BP_PlayerBase_C|SetEquipWeapon _asbp_player_base _output_get_4))
      (Variables|/Game/Characters/GameplayAbilitySystem/character/BP_PlayerBase.BP_PlayerBase_C|SetCurrentWeaponInt _asbp_player_base (Math|Conversions|ToInteger(Byte) (Variables|BP_PickUPComponent_C|GetWeaponName _output_get_5)))
      (Rendering|SetVisibility (Variables|/Game/Characters/GameplayAbilitySystem/character/BP_PlayerBase.BP_PlayerBase_C|GetSecondaryWeapon _asbp_player_base) true false)))
  (if (Pawn|IsLocallyControlled _asbp_player_base)
    (Development|PrintString (Utilities|GetDisplayName (Variables|/Script/Engine.Character|GetMesh _asbp_player_base)) true true "(R=1.000000,G=0.603604,B=0.013854,A=1.000000)")
    (switch Utilities|FlowControl|Switch|SwitchonE_WeaponType (Variables|Default|GetWeaponName)
      (:NewEnumerator0
        (Ability|SendGameplayEventtoActor (Variables|Default|GetAs%20BP%20Player%20Base) "(TagName=\"Event.ActiveAbility.EquipWeapon\")" (Utilities|Struct|MakeGameplayEventData "(GameplayTags=((TagName=\"Weapon.Range.Virtus\")))")))
      (:NewEnumerator1
        (Ability|SendGameplayEventtoActor (Variables|Default|GetAs%20BP%20Player%20Base) "(TagName=\"Event.ActiveAbility.EquipWeapon\")" (Utilities|Struct|MakeGameplayEventData "(GameplayTags=((TagName=\"Weapon.Range.Rifle\")))")))
      (:NewEnumerator2
        (Ability|SendGameplayEventtoActor (Variables|Default|GetAs%20BP%20Player%20Base) "(TagName=\"Event.ActiveAbility.EquipWeapon\")" (Utilities|Struct|MakeGameplayEventData "(GameplayTags=((TagName=\"Weapon.Range.Virtus\")))"))))
    (else
      ;[0.15 0.15 0.15 0.5] 服务器有延迟.
      (Utilities|FlowControl|Delay 0.1)
      (Development|PrintString (Utilities|String|ToString(Name) _socketname) true true "(R=0.000682,G=1.000000,B=0.120868,A=1.000000)")
      (bind _returnvalue (Transformation|AttachComponentToComponent (Variables|/Script/Engine.Character|GetMesh _asbp_player_base) _socketname "SnapToTarget" "SnapToTarget" "SnapToTarget" true))
      (Development|PrintString "True" _returnvalue true "(R=1.000000,G=0.143952,B=0.152546,A=1.000000)"))))

(event EventTick
  (params (DeltaSeconds :type Float%20%28single-precision%29)))