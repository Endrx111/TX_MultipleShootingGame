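; First-person player character that handles Enhanced Input movement, look, sprint, aiming and firing.
; Tick aligns the arms to control rotation, derives an Idle/Walk/Run/Aim state from input and velocity, sets walk speed and prints debug values.
; That state also scales look sensitivity and blocks firing while running.
; BeginPlay attaches a spawned VIRTUS weapon to the arms; aiming interpolates camera FOV, with a timer event for restoring it.
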(event Custom|OutFov
  (bind _returnvalue (Utilities|Time|GetWorldDeltaSeconds))
  (bind _camera (Variables|Default|GetCamera))
  (bind _defaultfov (Variables|Default|GetDefaultFov))
  (bind _fieldofview (Variables|/Script/Engine.CameraComponent|GetFieldOfView _camera))
  (bind _returnvalue_2 (Math|Interpolation|FInterpTo _fieldofview _defaultfov _returnvalue 8.0))
  (Camera|SetFieldOfView _camera _returnvalue_2)
  (if (Math|Float|NearlyEqual(Float) _returnvalue_2 (Variables|Default|GetDefaultFov) 0.1)
    (Utilities|Time|ClearandInvalidateTimerbyHandle (Variables|Default|GetOutFovHandle))))

(event Input|EnhancedActionEvents|EnhancedInputActionIA_Run
  (params (ActionValue :type Boolean) (ElapsedSeconds :type Float%20%28double-precision%29) (TriggeredSeconds :type Float%20%28double-precision%29) (InputAction :type Input%20Action%20Object%20Reference :default "/Game/Code/Player/System/Input/IA_Run.IA_Run"))
  (:Triggered
    (Variables|Default|SetWant%20to%20Run true))
  (:Completed
    (Variables|Default|SetWant%20to%20Run false)))

(event Input|EnhancedActionEvents|EnhancedInputActionIA_Move
  (params (ActionValue :type Vector%202D%20Structure) (ElapsedSeconds :type Float%20%28double-precision%29) (TriggeredSeconds :type Float%20%28double-precision%29) (InputAction :type Input%20Action%20Object%20Reference :default "/Game/Code/Player/System/Input/IA_Move.IA_Move"))
  (bind (_x _y) (Math|Vector2D|BreakVector2D ActionValue))
  (:Triggered
    (bind _output_get (Variables|Default|SetMoveX _x))
    (Pawn|Input|AddMovementInput (Math|Vector|GetForwardVector (Math|Rotator|MakeRotator 0.0 0.0 (.yaw (Pawn|GetControlRotation :!class /Script/Engine.Pawn)))) _output_get false)
    (bind _output_get_2 (Variables|Default|SetMoveY _y))
    (Pawn|Input|AddMovementInput (Math|Vector|GetRightVector (Math|Rotator|MakeRotator 0.0 0.0 (.yaw (Pawn|GetControlRotation :!class /Script/Engine.Pawn)))) _output_get_2 false))
  (:Completed
    (Variables|Default|SetMoveX 0.0)
    (Variables|Default|SetMoveY 0.0)))

(event Input|EnhancedActionEvents|EnhancedInputActionIA_Look
  (params (ActionValue :type Vector%202D%20Structure) (ElapsedSeconds :type Float%20%28double-precision%29) (TriggeredSeconds :type Float%20%28double-precision%29) (InputAction :type Input%20Action%20Object%20Reference :default "/Game/Code/Player/System/Input/IA_Look.IA_Look"))
  (bind (_x _y) (Math|Vector2D|BreakVector2D ActionValue))
  (bind _mousesensitive (Variables|Default|GetMouseSensitive))
  ;[0.15 0.15 0.15 0.5] 已经获取到鼠标的旋转
  ;[0.15 0.15 0.15 0.5] 因为x旋转绕y轴旋转
  (Pawn|Input|AddControllerYawInput (* _x (CallFunction|UPdateScopeSensitive) _mousesensitive))
  (Pawn|Input|AddControllerPitchInput (* _y (CallFunction|UPdateScopeSensitive) _mousesensitive)))

(event Input|EnhancedActionEvents|EnhancedInputActionIA_Aim
  (params (ActionValue :type Boolean) (ElapsedSeconds :type Float%20%28double-precision%29) (TriggeredSeconds :type Float%20%28double-precision%29) (InputAction :type Input%20Action%20Object%20Reference :default "/Game/Code/Player/System/Input/IA_Aim.IA_Aim"))
  (bind _returnvalue (Utilities|Time|GetWorldDeltaSeconds))
  (bind _camera (Variables|Default|GetCamera))
  (:Triggered
    (Variables|Default|SetWant%20to%20Aim true)
    (Camera|SetFieldOfView _camera (Math|Interpolation|FInterpTo (Variables|/Script/Engine.CameraComponent|GetFieldOfView _camera) 75.0 _returnvalue 8.0))
    (Utilities|Time|ClearandInvalidateTimerbyHandle (Variables|Default|GetOutFovHandle)))
  (:Completed
    (Variables|Default|SetWant%20to%20Aim false)
    (bind _returnvalue_2 (Utilities|Time|SetTimerbyEvent (delegate Custom|OutFov) _returnvalue))
    (Variables|Default|SetOutFovHandle _returnvalue_2)))

(event Input|EnhancedActionEvents|EnhancedInputActionIA_Fire
  (params (ActionValue :type Boolean) (ElapsedSeconds :type Float%20%28double-precision%29) (TriggeredSeconds :type Float%20%28double-precision%29) (InputAction :type Input%20Action%20Object%20Reference :default "/Game/Code/Player/System/Input/IA_Fire.IA_Fire"))
  (:Started
    (if (not (Variables|Default|GetIsFiring))
      (if (not (Variables|Default|GetIsDead))
        (if (Utilities|Enum|NotEqual(Enum) (Variables|Default|GetE_PlayerState) "NewEnumerator2")
          (Variables|Default|SetIsFiring true)
          (Default|StartWeaponFire (Variables|Default|GetCurrentWeapon))))))
  (:Completed
    (Default|StopFire (Variables|Default|GetCurrentWeapon))
    (Variables|Default|SetIsFiring false)))

(event EventBeginPlay
  (bind _as玩家控制器 (Utilities|Casting|CastToPlayerController (Pawn|GetController)))
  (Input|AddMappingContext (PlayerController|LocalPlayerSubsystems|GetEnhancedInputLocalPlayerSubsystem _as玩家控制器) "/Game/Code/Player/System/Input/IMC_FPSInput.IMC_FPSInput" 10 "(bIgnoreAllPressedKeysUntilRelease=True,bForceImmediately=False,bNotifyUserSettings=False)")
  (CallFunction|SpawnWeapon self "/Game/Code/Weapon/BP_VIRTUS.BP_VIRTUS_C")
  (CallFunction|UpdateDeafultFov))

(event Collision|EventActorBeginOverlap
  (params (OtherActor :type Actor%20Object%20Reference)))

(event EventTick
  (params (DeltaSeconds :type Float%20%28single-precision%29))
  (bind _returnvalue (Pawn|GetControlRotation :!class /Script/Engine.Pawn))
  (Transformation|SetWorldRotation (Variables|Default|GetArm) (Math|Rotator|MakeRotator 0.0 (.pitch _returnvalue) (.yaw _returnvalue)) false false)
  (CallFunction|UpdatePlayerState)
  (Development|PrintString (Utilities|String|EnumtoString (Variables|Default|GetE_PlayerState)) true true "(R=0.000000,G=0.660000,B=1.000000,A=1.000000)" 0.0)
  (CallFunction|UpdateMoveSpeed)
  (Development|PrintString (Utilities|String|ToString(Float) (Variables|/Script/Engine.CharacterMovementComponent|GetMaxWalkSpeed (Variables|Character|GetCharacterMovement))) true true "(R=0.000000,G=0.660000,B=1.000000,A=1.000000)" 0.0))

(fn ConstructionScript)

(fn UpdatePlayerState
  (if (Variables|Default|GetWant%20to%20Aim)
    (Variables|Default|SetE_PlayerState "NewEnumerator3")
    (elif (> (Variables|Default|GetMoveX) 0.0)
      (if (Variables|Default|GetWant%20to%20Run)
        (Variables|Default|SetE_PlayerState "NewEnumerator2")
        (else
          (Variables|Default|SetE_PlayerState "NewEnumerator1")))
      (elif (> (Math|Vector|VectorLength (Variables|/Script/Engine.MovementComponent|GetVelocity (Variables|Character|GetCharacterMovement))) 0.0)
        (Variables|Default|SetE_PlayerState "NewEnumerator1")
        (else
          (Variables|Default|SetE_PlayerState "NewEnumerator0"))))))

(fn UpdateMoveSpeed
  (Variables|/Script/Engine.CharacterMovementComponent|SetMaxWalkSpeed (Variables|Character|GetCharacterMovement) (Utilities|Select :Index (Variables|Default|GetE_PlayerState) :NewEnumerator0 4e+02 :NewEnumerator1 4e+02 :NewEnumerator2 6e+02 :NewEnumerator3 265.0 :NewEnumerator4 0.0)))

(fn SpawnWeapon
  (params (Class :type Actor%20Class%20Reference))
  (bind _returnvalue (Game|SpawnActorfromClass Class (Math|Transform|MakeTransform "0, 0, 0" "0, 0, 0" "1.000000,1.000000,1.000000") "Undefined" "MultiplyWithRoot" self 0))
  (bind _asbp_weapon_base (Utilities|Casting|CastToBP_WeaponBase _returnvalue))
  (bind _output_get (Variables|Default|SetCurrentWeapon _asbp_weapon_base))
  (Transformation|AttachComponentToComponent _output_get (Variables|Default|GetArm) "Weapon" "KeepRelative" "KeepRelative" "KeepRelative" true))

(fn UpdateDeafultFov
  (Variables|Default|SetDefaultFov (Variables|/Script/Engine.CameraComponent|GetFieldOfView (Variables|Default|GetCamera))))

(fn UPdateScopeSensitive
  (return (Utilities|Select :Index (Variables|Default|GetE_PlayerState) :NewEnumerator0 1.0 :NewEnumerator1 1.0 :NewEnumerator2 1.0 :NewEnumerator3 0.6 :NewEnumerator4 0.0)))