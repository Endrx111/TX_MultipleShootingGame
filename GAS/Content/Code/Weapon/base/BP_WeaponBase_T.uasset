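; Base weapon actor for an automatic hitscan rifle, with MCX VIRTUS assets hard-coded.
; An Idle/Firing/Reloading state gates a looping fire timer and montage-only reload; ammo counts are checked but never changed.
; Each shot plays player-state montages, muzzle flash, sound, casing and recoil, then line-traces from camera center.
; Physical surface type selects impact effects, sound and decal; Enemy reuses Wood because blood effects are disconnected, and no damage is applied.
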(event Custom|FireInternal
  (bind _idle (Variables|Default|GetIdle))
  (bind _weapon (Variables|Default|GetWeapon))
  (bind _player (Variables|Default|GetPLayer))
  (bind _player_2 (Variables|Default|GetPLayer))
  (bind _returnvalue (Transformation|GetSocketTransform _weapon "casing" "RTS_World"))
  (bind _followcamera (Variables|/Game/Characters/GameplayAbilitySystem/character/BP_Player_T.BP_Player_T_C|GetFollowCamera _player_2))
  (bind _returnvalue_2 (Transformation|GetWorldLocation _followcamera))
  (bind _notifyname (Animation|Montage|PlayMontage (Variables|/Game/Characters/GameplayAbilitySystem/character/BP_Player_T.BP_Player_T_C|Gethan (Variables|Default|GetPLayer)) (Utilities|Select :Index (Variables|/Game/Characters/GameplayAbilitySystem/character/BP_Player_T.BP_Player_T_C|GetE_PlayerState (Variables|Default|GetPLayer)) :NewEnumerator0 _idle :NewEnumerator1 (Variables|Default|GetWalk) :NewEnumerator2 0 :NewEnumerator3 (Variables|Default|GetAim) :NewEnumerator4 0))
    (:then
      (Development|PrintString (Utilities|String|ToString(Object) _idle))
      (Animation|Montage|PlayMontage (Variables|Default|GetWeapon) (Utilities|Select :Index (Variables|/Game/Characters/GameplayAbilitySystem/character/BP_Player_T.BP_Player_T_C|GetE_PlayerState (Variables|Default|GetPLayer)) :NewEnumerator0 (Variables|Default|Getweapon_Idle_0) :NewEnumerator1 (Variables|Default|Getweapon_Walk_0) :NewEnumerator2 0 :NewEnumerator3 (Variables|Default|Getweapon_Aim_0) :NewEnumerator4 0)
        (:then
          (Audio|PlaySound2D "/Game/Code/Weapon/MetaSound/MS_VIRTUS.MS_VIRTUS" 1.0 1.0 0.0 0 0)
          (Niagara|SpawnSystemAttached "/Game/ShotSystem/Shot_VFX/VIRTUS_MuzzleFlash.VIRTUS_MuzzleFlash" (Variables|Default|GetBarrel%28Cancel%20collision) "Muzzle" "0, 0, 0" "0, 0, 0" "KeepRelativeOffset" false)
          (Game|SpawnActorfromClass "/Game/Code/Weapon/BP_Casing.BP_Casing_C" (Math|Transform|MakeTransform (.location _returnvalue) (.rotation _returnvalue) "1.000000,1.000000,1.000000") "Undefined" "MultiplyWithRoot" 0 0)
          (Pawn|Input|AddControllerPitchInput _player -0.4)
          (Pawn|Input|AddControllerYawInput _player (Math|Random|RandomFloatinRange -0.1 0.1))
          ;[0.15 0.15 0.15 0.5] 从屏幕正中间射击出去射线
          (bind _outhit (Collision|LineTraceByChannel _returnvalue_2 (+ _returnvalue_2 (* (Math|Vector|GetForwardVector _followcamera) 10000)) "TraceTypeQuery1" false 0 "None"))
          (if (.bBlockingHit (Collision|BreakHitResult _outhit))
            (Variables|Default|SetLocation (.Location (Collision|BreakHitResult _outhit)))
            (switch Utilities|FlowControl|Switch|SwitchonEPhysicalSurface (Variables|/Script/PhysicsCore.PhysicalMaterial|GetSurfaceType (.PhysMat (Collision|BreakHitResult _outhit)))
              (:SurfaceType_Default
                ;[0.15 0.15 0.15 0.5] 弹道差分
                (Niagara|SpawnSystematLocation "/Game/ShotSystem/Shot_VFX/FX_SquibConcrete.FX_SquibConcrete" (Variables|Default|GetLocation) :!label _label)
                (Audio|PlaySoundatLocation "/Game/ShotSystem/Shot_SFX/SFX_Vefects_Shots_Squib_Concrete_Cue.SFX_Vefects_Shots_Squib_Concrete_Cue" (Variables|Default|GetLocation) "0, 0, 0" 1.6 1.0 0.0 0 0 0 0)
                (bind _returnvalue_3 (Game|SpawnActorfromClass "/Game/Decals/BP_BulletDecal.BP_BulletDecal_C" (Math|Transform|MakeTransform "0, 0, 0" (Math|Rotator|MakeRotfromX (.Normal (Collision|BreakHitResult _outhit))) "0.400000,0.400000,0.400000") "Undefined" "MultiplyWithRoot" 0 0))
                (Rendering|Components|Decal|SetDecalMaterial (Variables|/Game/Decals/BP_BulletDecal.BP_BulletDecal_C|GetBulletDecal _returnvalue_3) "/Game/Decals/Materials/MI_VFX_BulletDecal_Concrete.MI_VFX_BulletDecal_Concrete"))
              (:SurfaceType1
                (Niagara|SpawnSystematLocation "/Game/ShotSystem/Shot_VFX/FX_SquibWood.FX_SquibWood" (Variables|Default|GetLocation) (Math|Rotator|MakeRotfromX (.Normal (Collision|BreakHitResult _outhit))) :!label _label_2)
                (Audio|PlaySoundatLocation "/Game/ShotSystem/Shot_SFX/SFX_Vefects_Shots_Squib_Metal_Cue.SFX_Vefects_Shots_Squib_Metal_Cue" (Variables|Default|GetLocation) "0, 0, 0" 1.6 1.0 0.0 0 0 0 0)
                (bind _returnvalue_4 (Game|SpawnActorfromClass "/Game/Decals/BP_BulletDecal.BP_BulletDecal_C" (Math|Transform|MakeTransform (Variables|Default|GetLocation) (Math|Rotator|MakeRotfromX (.Normal (Collision|BreakHitResult _outhit))) "0.400000,0.400000,0.400000") "Undefined" "MultiplyWithRoot" 0 0))
                (Rendering|Components|Decal|SetDecalMaterial (Variables|/Game/Decals/BP_BulletDecal.BP_BulletDecal_C|GetBulletDecal _returnvalue_4) "/Game/Decals/Materials/MI_VFX_BulletDecal_Wood.MI_VFX_BulletDecal_Wood"))
              (:SurfaceType2
                ;[0.15 0.15 0.15 0.5] 弹道差分
                (Niagara|SpawnSystematLocation "/Game/ShotSystem/Shot_VFX/FX_SquibDirt.FX_SquibDirt" (Variables|Default|GetLocation) (Math|Rotator|MakeRotfromX (.Normal (Collision|BreakHitResult _outhit))))
                (Audio|PlaySoundatLocation "/Game/ShotSystem/Shot_SFX/SFX_Vefects_Shots_Squib_Dirt_Cue.SFX_Vefects_Shots_Squib_Dirt_Cue" (Variables|Default|GetLocation) "0, 0, 0" 1.6 1.0 0.0 0 0 0 0)
                (bind _returnvalue_5 (Game|SpawnActorfromClass "/Game/Decals/BP_BulletDecal.BP_BulletDecal_C" (Math|Transform|MakeTransform (Variables|Default|GetLocation) (Math|Rotator|MakeRotfromX (.Normal (Collision|BreakHitResult _outhit))) "0.400000,0.400000,0.400000") "Undefined" "MultiplyWithRoot" 0 0))
                (Rendering|Components|Decal|SetDecalMaterial (Variables|/Game/Decals/BP_BulletDecal.BP_BulletDecal_C|GetBulletDecal _returnvalue_5) "/Game/ShotSystem/Shot_VFX/Shared/Materials/SmokeBased/MI_VFX_DirtBurst01.MI_VFX_DirtBurst01"))
              (:SurfaceType3
                (Niagara|SpawnSystematLocation "/Game/ShotSystem/Shot_VFX/FX_SquibMetal.FX_SquibMetal" (Variables|Default|GetLocation) (Math|Rotator|MakeRotfromX (.Normal (Collision|BreakHitResult _outhit))))
                (Audio|PlaySoundatLocation "/Game/ShotSystem/Shot_SFX/SFX_Vefects_Shots_Squib_Metal_Cue.SFX_Vefects_Shots_Squib_Metal_Cue" (Variables|Default|GetLocation) "0, 0, 0" 1.6 1.0 0.0 0 0 0 0)
                (bind _returnvalue_6 (Game|SpawnActorfromClass "/Game/Decals/BP_BulletDecal.BP_BulletDecal_C" (Math|Transform|MakeTransform (Variables|Default|GetLocation) (Math|Rotator|MakeRotfromX (.Normal (Collision|BreakHitResult _outhit))) "0.400000,0.400000,0.400000") "Undefined" "MultiplyWithRoot" 0 0))
                (Rendering|Components|Decal|SetDecalMaterial (Variables|/Game/Decals/BP_BulletDecal.BP_BulletDecal_C|GetBulletDecal _returnvalue_6) "/Game/Decals/Materials/MI_VFX_BulletDecal_Metal.MI_VFX_BulletDecal_Metal"))
              (:SurfaceType4
                (goto _label_2))
              (:SurfaceType5
                (goto _label)))))))))

(event Custom|StopFire
  (switch Utilities|FlowControl|Switch|SwitchonE_WeaponState (Variables|Default|GetWeaponState)
    (:NewEnumerator0
      _)
    (:NewEnumerator1
      _))
  (Utilities|Time|ClearandInvalidateTimerbyHandle (Variables|Default|GetFireTimeHandle))
  (Variables|Default|SetWeaponState "NewEnumerator0"))

(event Custom|Reload
  (switch Utilities|FlowControl|Switch|SwitchonE_WeaponState (Variables|Default|GetWeaponState)
    (:NewEnumerator0
      (if (Math|Boolean|NANDBoolean (< (Variables|Default|GetCurrentAmmo) (Variables|Default|GetMagSize)) (> (Variables|Default|GetTotalAmmo) 0))
        (Variables|Default|SetWeaponState "NewEnumerator2")
        (Animation|Montage|PlayMontage (Variables|Default|GetWeapon) "/Game/XL_FPSPack/Weapons/MCX-VIRTUS/Animation/Weapon/Weapon_MCX-VIRTUS_Reload_Empty_Montage.Weapon_MCX-VIRTUS_Reload_Empty_Montage"
          (:then
            (Animation|Montage|PlayMontage (Variables|/Game/Characters/GameplayAbilitySystem/character/BP_Player_T.BP_Player_T_C|Gethan (Variables|Default|GetPLayer)) "/Game/XL_FPSPack/Weapons/MCX-VIRTUS/Animation/Player/Player_MCX-VIRTUS_Reload_Empty_Montage.Player_MCX-VIRTUS_Reload_Empty_Montage"
              (:then
                (Audio|PlaySound2D "/Game/XL_FPSPack/Weapons/MCX-VIRTUS/Sound/Foley/SW_MCX-VIRTUS_Reload_Empty_Foley.SW_MCX-VIRTUS_Reload_Empty_Foley" 1.0 1.0 0.0 0 0))
              (:OnCompleted
                (Variables|Default|SetWeaponState "NewEnumerator0" :!label _label))
              (:OnInterrupted
                (goto _label)))))))))

(event EventBeginPlay)

(event Collision|EventActorBeginOverlap
  (params (OtherActor :type Actor%20Object%20Reference)))

(event EventTick
  (params (DeltaSeconds :type Float%20%28single-precision%29)))

(event EventStartWeaponT
  (params (Player :type BP%20Player%20T%20Object%20Reference))
  (Variables|Default|SetPLayer Player)
  (switch Utilities|FlowControl|Switch|SwitchonE_WeaponState (Variables|Default|GetWeaponState)
    (:NewEnumerator0
      (if (> (Variables|Default|GetCurrentAmmo) 0)
        (CallFunction|FireInternal)
        (bind _returnvalue (Utilities|Time|SetTimerbyEvent (delegate Custom|FireInternal) (Variables|Default|GetFIreRate) true))
        (Variables|Default|SetFireTimeHandle _returnvalue)
        (Variables|/Game/Characters/GameplayAbilitySystem/character/BP_Player_T.BP_Player_T_C|SetIsFiring (Variables|Default|GetPLayer) true)
        (Variables|Default|SetWeaponState "NewEnumerator1")))))

(event EventStartWeaponFire
  (params (PLayer :type BP%20Player%20Base%20Object%20Reference)))

(fn ConstructionScript)

(fn GetAimSocket
  (bind _output_get (Variables|Default|SetAimSocketLOcation (Transformation|GetSocketLocation (Variables|Default|GetWeapon) "Weapon")))
  (return _output_get))